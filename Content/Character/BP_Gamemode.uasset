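; BP_Gamemode watches plant and seed progress on a looping one-second timer.
; When a BP_Plant_Child2 exists it plays audio once; a BP_Plant_Child5 lowers the hero's gravity scale and sets a new jump velocity.
; It also prints debug counts and respawns a first BP_Seed at the first TargetPoint found when no plants, seeds or held seed remain, preventing a dead end.
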(event `self.ReceiveBeginPlay`
  (`KismetSystemLibrary.K2_SetTimerDelegate` (delegate `CheckGameOver`) 1.0 true))

(event `CheckGameOver`
  (bind _outactors (`GameplayStatics.GetAllActorsOfClass` "/Game/Objects/Plants/BP_Plant.BP_Plant_C"))
  (`|ExecutionSequence`
    (:`then_0`
      (if (not (`self.Child2OK`))
        (for _array_element _outactors
          (if (== (`GameplayStatics.GetObjectClass` _array_element) "/Game/Objects/Plants/BP_Plant_Child2.BP_Plant_Child2_C")
            (`/Engine/EditorBlueprintResources/StandardMacros.DoOnce` false
              (:`Completed`
                (set `self.Child2OK` true)
                (`AudioComponent.Play` (`self.Audio`) 0.0)))))))
    (:`then_1`
      (if (not (`self.Child5OK`))
        (for _array_element_2 _outactors
          (if (== (`GameplayStatics.GetObjectClass` _array_element_2) "/Game/Objects/Plants/BP_Plant_Child5.BP_Plant_Child5_C")
            (`/Engine/EditorBlueprintResources/StandardMacros.DoOnce` false
              (:`Completed`
                (set `self.Child5OK` false)
                (`KismetSystemLibrary.PrintString` "Hello")
                (bind _asbp_hero_n (cast `/Game/Character/BP_HeroN` (`GameplayStatics.GetPlayerPawn` 0)))
                (bind _charactermovement (`Character.CharacterMovement` _asbp_hero_n))
                (set `CharacterMovementComponent.GravityScale` 0.5 _charactermovement)
                (set `CharacterMovementComponent.JumpZVelocity` 800.0 _charactermovement)))))))
    (:`then_2`
      (bind _outactors_2 (`GameplayStatics.GetAllActorsOfClass` "/Game/Objects/BP_Seed.BP_Seed_C"))
      (bind _asbp_hero_n_2 (cast `/Game/Character/BP_HeroN` (`GameplayStatics.GetPlayerPawn` 0)))
      (bind _returnvalue (`KismetArrayLibrary.Array_Length` _outactors))
      (bind _returnvalue_2 (`KismetArrayLibrary.Array_Length` _outactors_2))
      (bind _seedisinhand (`/Game/Character/BP_HeroN.SeedIsInHand` _asbp_hero_n_2))
      (`KismetSystemLibrary.PrintString` (`KismetStringLibrary.Concat_StrStr` "Plants " (`KismetStringLibrary.Conv_IntToString` _returnvalue) " \nSeeds " (`KismetStringLibrary.Conv_IntToString` _returnvalue_2) " \nHero has seed in hand " (`KismetStringLibrary.Conv_BoolToString` _seedisinhand)) true true (struct :`R` 1.0 :`G` 1.0 :`B` 1.0 :`A` 1.0) 0.5)
      (if (and (== _returnvalue 0) (== _returnvalue_2 0) (not _seedisinhand))
        ;[1 1 1] Pop 1st seed
        (bind _outactors_3 (`GameplayStatics.GetAllActorsOfClass` "/Script/Engine.TargetPoint"))
        (`|SpawnActorFromClass` "/Game/Objects/BP_Seed.BP_Seed_C" (`self.GetTransform` (`KismetArrayLibrary.Array_Get` _outactors_3)) "Undefined" "OverrideRootScale" null false 1 true)))))

(fn `UserConstructionScript`)