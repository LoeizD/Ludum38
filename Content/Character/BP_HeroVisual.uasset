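; BP_HeroVisual is the visual actor for a hero: an animated skeletal mesh that can show a carried seed.
; The construction script adds the Seed static mesh and snaps it to the "joint7" socket.
; Custom events loop the Run or Idle animation directly without an AnimBP, toggle seed visibility, and set the actor's transform with an XY offset, passing only roll and yaw for rotation.
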(event `PlayAnimation`
  (params (Run :type Boolean))
  (`SkeletalMeshComponent.PlayAnimation` (`self.SkeletalMesh`) (select `bool` Run :`false` "/Game/Character/HeroAnim/Idle.Idle" :`true` "/Game/Character/HeroAnim/Run.Run" :!type "AnimationAsset Object Reference") true))

(event `SetLocAndRot`
  (params (NewLocation :type "Vector Structure") (NewRotation :type "Rotator Structure"))
  (bind (_offset_x _offset_y) (`KismetMathLibrary.BreakVector2D` (`self.Offset`)))
  (`self.K2_SetActorLocationAndRotation` (+ NewLocation (`KismetMathLibrary.MakeVector` _offset_x _offset_y)) (`KismetMathLibrary.MakeRotator` NewRotation_Roll 0.0 NewRotation_Yaw)))

(event `SeeSeed`
  (params (Visibility :type Boolean))
  (`SceneComponent.SetVisibility` (`self.Seed`) Visibility false))

(fn `UserConstructionScript`
  (bind _returnvalue (`AddComponent|NODE_AddStaticMeshComponent-0`))
  (bind _output_get (set `self.Seed` _returnvalue))
  (`SceneComponent.K2_AttachToComponent` _output_get (`self.SkeletalMesh`) "joint7" "SnapToTarget" "SnapToTarget" "KeepRelative" true))