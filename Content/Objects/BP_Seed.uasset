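; BP_Seed is a physics seed that pops out along its forward vector and can be grabbed, thrown or left to grow into a plant.
; Tick runs a state machine that follows the hand anchor when held and uses zero velocity to detect rest.
; A seed resting on the ground plants itself after a timer, while a thrown one plants on floor overlap.
; Planting spawns BP_Plant_Child1 and an SFX actor, then destroys the seed.
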(event `self.ReceiveBeginPlay`
  (bind _seedcollider (`self.SeedCollider`))
  ;[0.6063 1 0] BEGIN PLAY
  (`parent.ReceiveBeginPlay`)
  (`PrimitiveComponent.AddImpulse` _seedcollider (* (`KismetMathLibrary.GetForwardVector` (`SceneComponent.K2_GetComponentRotation` _seedcollider)) (* (`PrimitiveComponent.GetMass` _seedcollider) 800.0)) "None" false)
  (`self.InitAutoPlantingTimer`)
  (if (not (`self.HasBeenGrabedAtLeastOnce`))
    ;[1 1 1] SFX Pop from plant
    (`AudioComponent.Play` (`self.PopSeed`) 0.0)))

(event `self.ReceiveTick`
  (params (DeltaSeconds :type "Float (single-precision)"))
  (bind _seedcollider (`self.SeedCollider`))
  ;[0.09175 1 0] EVENT TICK
  (if (not (`self.IsPlant`)) :!pinned true
    (switch `/Game/Objects/E_SeedStates` (`self.State`)
      (:`NewEnumerator0`
        (`self.TestVelocity`
          (:`Stop`
            (set `self.State` "NewEnumerator3"))))
      (:`NewEnumerator3`
        (`self.TestVelocity`
          (:`Stop`
            ;[1 1 1] AutoPlanting timer
            (bind _output_get (set `self.AutoPlantingTimerCurrent` (- (`self.AutoPlantingTimerCurrent`) (`GameplayStatics.GetWorldDeltaSeconds`))))
            (if (<= _output_get 0.0)
              (`self.SpawnPlant`)))
          (:`Moving`
            (`self.InitAutoPlantingTimer`)
            (if (`self.HasBeenGrabedAtLeastOnce`)
              (set `self.State` "NewEnumerator4")
              (else
                (set `self.State` "NewEnumerator0"))))))
      (:`NewEnumerator1`
        (`self.InitAutoPlantingTimer`)
        (`self.FixSeedInHand`)
        (set `self.HasBeenGrabedAtLeastOnce` true))
      (:`NewEnumerator2`
        ;[1 1 1] Enable phys & gravity
        (`PrimitiveComponent.SetSimulatePhysics` _seedcollider true)
        (`PrimitiveComponent.SetEnableGravity` _seedcollider true)
        (set `self.State` "NewEnumerator4")))))

(event `SeedGrabed`
  (params (HandAnchor :type "SceneComponent Object Reference"))
  (bind _seedcollider (`self.SeedCollider`))
  (set `self.TempHand` HandAnchor)
  ;[1 1 1] DIsable phys & gravity
  (`PrimitiveComponent.SetSimulatePhysics` _seedcollider false)
  (`PrimitiveComponent.SetEnableGravity` _seedcollider false)
  (set `self.State` "NewEnumerator1"))

(event `self.TriggerFloor.OnComponentBeginOverlap`
  (params (OverlappedComponent :type "PrimitiveComponent Object Reference") (OtherActor :type "Actor Object Reference") (OtherComp :type "PrimitiveComponent Object Reference") (OtherBodyIndex :type Integer) (bFromSweep :type Boolean) (SweepResult :type "HitResult Structure (by ref)"))
  ;[1 1 1] SFX Fall in grass
  (`AudioComponent.Play` (`self.FallGrass`) 0.0)
  (if (`|EnumEquality` (`self.State`) "NewEnumerator4")
    (`self.SpawnPlant`)))

(fn `FixSeedInHand`
  (bind (_returnvalue_location _returnvalue_rotation) (`KismetMathLibrary.BreakTransform` (`SceneComponent.K2_GetComponentToWorld` (`self.TempHand`))))
  (`SceneComponent.K2_SetWorldLocationAndRotation` (`self.SeedCollider`) _returnvalue_location _returnvalue_rotation false false))

(fn `InitAutoPlantingTimer`
  (set `self.AutoPlantingTimerCurrent` (`self.AutoPlantingTimer`)))

(fn `SpawnPlant`
  (bind (_returnvalue_location _returnvalue_rotation) (`KismetMathLibrary.BreakTransform` (`SceneComponent.K2_GetComponentToWorld` (`self.SeedCollider`))))
  (bind (_returnvalue_x _returnvalue_y) (`KismetMathLibrary.BreakVector` (`SceneComponent.K2_GetComponentLocation` (`self.SeedCollider`))))
  (set `self.IsPlant` true)
  ;[1 1 1] SFX Pop
  (`|SpawnActorFromClass` "/Game/Sounds/BP_SFXPlantSpawn.BP_SFXPlantSpawn_C" (`KismetMathLibrary.MakeTransform` _returnvalue_location _returnvalue_rotation) "Undefined" "OverrideRootScale")
  (`|SpawnActorFromClass` "/Game/Objects/BP_Plant_Child1.BP_Plant_Child1_C" (`KismetMathLibrary.MakeTransform` (`KismetMathLibrary.MakeVector` _returnvalue_x _returnvalue_y)) "Undefined" "OverrideRootScale" null true)
  (`self.K2_DestroyActor`))

(fn `TestIfVelocity0`
  (returns (Velocity0 :type Boolean))
  (bind _returnvalue (`PrimitiveComponent.GetPhysicsLinearVelocity` (`self.SeedCollider`) "None"))
  (return (== (`KismetMathLibrary.VSize` _returnvalue) 0.0)))

(fn `UserConstructionScript`
  (`parent.UserConstructionScript`))