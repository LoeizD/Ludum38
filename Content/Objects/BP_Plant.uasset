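; BP_Plant is a plant actor that withers over time, can be watered, and spreads seeds.
; Tick shrinks the visual toward quarter size as remaining life drains, destroying the actor below zero; Water restores life up to the maximum.
; From BeginPlay, a looped random Delay spawns a limited number of inactive BP_Seed actors above the plant, randomly yawing AnchorRotation before each to vary SpawnSeedDirection.
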(event `self.ReceiveBeginPlay`
  (`parent.ReceiveBeginPlay`)
  (set `self.LifeRemaining` (`self.LifeMax`))
  ;[1 1 1] Spawn seed
  (`KismetSystemLibrary.Delay` (`KismetMathLibrary.RandomFloatInRange` (`self.SeedSpawnTimeMin`) (`self.SeedSpawnTimeMax`)) :!label _label)
  (`self.SpawnSeed`)
  (bind _output_get (set `self.NumberOfSeeds` (- (`self.NumberOfSeeds`) 1)))
  (if (> _output_get 0)
    (goto _label)))

(event `self.ReceiveTick`
  (params (DeltaSeconds :type "Float (single-precision)"))
  (`self.ScaleVisualByLife`)
  (bind _newlife (`self.UpdateLife`))
  (`self.Death` _newlife))

(event `Water`
  (bind _returnvalue (+ (`self.LifeRemaining`) (`self.WaterAddTime`)))
  (set `self.LifeRemaining` (select `bool` (> _returnvalue (`self.LifeMax`)) :`false` _returnvalue :`true` (`self.LifeMax`))))

(fn `Death`
  (params (A :type "Float (double-precision)"))
  (if (< A 0.0)
    (`self.K2_DestroyActor`)))

(fn `ScaleVisualByLife`
  (bind _returnvalue (+ 0.25 (* (/ (`self.LifeRemaining`) (`self.LifeMax`)) 0.75)))
  (`SceneComponent.SetRelativeScale3D` (`self.Visual`) (`KismetMathLibrary.MakeVector` _returnvalue _returnvalue _returnvalue)))

(fn `SpawnSeed`
  (`SceneComponent.K2_SetRelativeRotation` (`self.AnchorRotation`) (`KismetMathLibrary.MakeRotator` 0.0 0.0 (`KismetMathLibrary.RandomFloatInRange` 0.0 360.0)) false false)
  (`|SpawnActorFromClass` "/Game/Objects/BP_Seed.BP_Seed_C" (`KismetMathLibrary.MakeTransform` (+ (`self.K2_GetActorLocation`) (* (`self.GetActorUpVector`) 50.0)) (`SceneComponent.K2_GetComponentRotation` (`self.SpawnSeedDirection`))) "Undefined" "OverrideRootScale"))

(fn `UpdateLife`
  (returns (NewLife :type "Float (double-precision)"))
  (bind _output_get (set `self.LifeRemaining` (- (`self.LifeRemaining`) (`GameplayStatics.GetWorldDeltaSeconds`))))
  (return _output_get))

(fn `UserConstructionScript`
  (`parent.UserConstructionScript`))