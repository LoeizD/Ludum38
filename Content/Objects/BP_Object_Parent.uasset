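; Base actor for objects in a tiled world that can copy itself across the surrounding tile grid.
; On BeginPlay it reads tile size and display distance from the first BP_Tiling actor.
; Replicate, unrelated to networking, spawns inactive instances of its own class at tile-spaced X/Y offsets, one tile beyond display distance, skipping the centre and storing them in Tiles.
; Nothing here calls Replicate, and the construction script's IsActive check is empty.
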(event `self.ReceiveBeginPlay`
  (bind _outactors (`GameplayStatics.GetAllActorsOfClass` "/Game/Levels/Tiling/BP_Tiling.BP_Tiling_C"))
  (bind _item (`KismetArrayLibrary.Array_Get` _outactors))
  (set `self.TileSize` (`/Game/Levels/Tiling/BP_Tiling.TileSize` _item))
  (set `self.DisplayDistance` (`/Game/Levels/Tiling/BP_Tiling.DisplayDistance` _item)))

(fn `Replicate`
  (bind (_returnvalue_x _returnvalue_y) (`KismetMathLibrary.BreakVector` (`self.K2_GetActorLocation`)))
  (bind _returnvalue (* (`self.TileSize`) 100.0))
  (bind _returnvalue_2 (+ (* (`self.DisplayDistance`) 2) 2))
  (for _index (range (+ _returnvalue_2 1))
    (for _index_2 (range (+ _returnvalue_2 1))
      (bind _returnvalue_3 (- (- _index_2 1) (`self.DisplayDistance`)))
      (bind _returnvalue_4 (- (- _index 1) (`self.DisplayDistance`)))
      (if (not (and (== _returnvalue_3 0) (== _returnvalue_4 0)))
        (bind _returnvalue_5 (`|SpawnActorFromClass` (`GameplayStatics.GetObjectClass` self) (`KismetMathLibrary.MakeTransform` (`KismetMathLibrary.MakeVector` (+ (* _returnvalue_4 _returnvalue) _returnvalue_x) (+ (* _returnvalue_3 _returnvalue) _returnvalue_y)) (struct) (1.0 1.0 1.0)) "Undefined" "OverrideRootScale"))
        (`KismetArrayLibrary.Array_Add` (`self.Tiles`) _returnvalue_5)))))

(fn `UserConstructionScript`
  (if (`self.IsActive`)
    _))