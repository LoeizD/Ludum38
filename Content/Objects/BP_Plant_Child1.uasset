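; BP_Plant_Child1 is a plant variant that inherits its behavior from a parent plant Blueprint, apparently BP_Plant.
; Its construction script calls the parent, then overrides plant index, maximum life, seed spawn timing, and the area degeneration value and radius.
; Seed spawn minimum and maximum times are equal, so any random interval between them becomes fixed.
; The event graph holds only disabled stubs, leaving all runtime logic to the parent.
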(fn `UserConstructionScript`
  (`parent.UserConstructionScript`)
  (set `self.PlantIndex` 1)
  (set `self.LifeMax` 50.0)
  (set `self.FirstSeedSpawnTime` 55.0)
  (set `self.SeedSpawnTimeMin` 25.0)
  (set `self.SeedSpawnTimeMax` 25.0)
  (set `self.AreaDegenValue` 0.25)
  (set `self.AreaRadius` 4.0))