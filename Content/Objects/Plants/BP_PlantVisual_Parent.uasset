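; Parent Blueprint for a plant's visual actor, which destroys itself on Tick once its Master reference is invalid.
; BeginPlay gathers flower child actors under Flowerz, and the first Tick applies the sphere's scale.
; UpdateTransform applies the stored transform and XY offset, then passes flower scale to each BP_Flower.
; Other functions drive the skeletal mesh's "Life" material parameter and remove the flowers, stopping further flower updates.
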(event `self.ReceiveBeginPlay`
  (set `self.InitSphereScale` false)
  (for _array_element (`SceneComponent.GetChildrenComponents` (`self.Flowerz`) false)
    (`KismetArrayLibrary.Array_Add` (`self.Flowers`) (`ChildActorComponent.ChildActor` (cast `ChildActorComponent` _array_element :!pure true)))))

(event `self.ReceiveTick`
  (params (DeltaSeconds :type "Float (single-precision)"))
  (bind _spherescale (`self.SphereScale`))
  (if (`self.InitSphereScale`)
    (`/Engine/EditorBlueprintResources/StandardMacros.IsValid` (`self.Master`)
      (:`Is Not Valid`
        (`KismetSystemLibrary.PrintString` "fail")
        (`self.K2_DestroyActor`)))
    (else
      (`SceneComponent.SetWorldScale3D` (`self.Sphere`) (`KismetMathLibrary.MakeVector` _spherescale _spherescale _spherescale))
      (set `self.InitSphereScale` true))))

(fn `KillFlower`
  (`self.SetLifeSpan` (`self.Flowers`) 0.01)
  (set `self.NoFlower` true))

(fn `UpdateMaterialParams`
  (params (Color :type "LinearColor Structure") (LifeState :type "Float (double-precision)"))
  (`MeshComponent.SetScalarParameterValueOnMaterials` (`self.SkeletalMesh`) "Life" LifeState))

(fn `UpdateTransform`
  (params (Transform :type "Transform Structure") (FlowerScale :type "Float (double-precision)"))
  (bind (_offsest_x _offsest_y) (`KismetMathLibrary.BreakVector2D` (`self.Offsest`)))
  (`SceneComponent.K2_SetRelativeTransform` (`self.Scale`) (`KismetMathLibrary.MakeTransform` (0.0 0.0 0.0) Transform_Rotation Transform_Scale) false false)
  (`self.K2_SetActorLocation` (+ Transform_Location (`KismetMathLibrary.MakeVector` _offsest_x _offsest_y)))
  (if (not (`self.NoFlower`))
    (for _array_element (`self.Flowers`)
      (`/Game/Objects/Plants/BP_Flower.UpdateFlower` (cast `/Game/Objects/Plants/BP_Flower` _array_element :!pure true) FlowerScale))))

(fn `UserConstructionScript`)