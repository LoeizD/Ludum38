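; BP_DropOfPiss is a physics-driven projectile for a single drop of urine.
; On BeginPlay it slightly randomizes the root's rotation for spread, then applies an impulse to its collision component along the actor's forward vector.
; Overlaps on that component only print a brief "wet" debug message, with no further gameplay effect in this Blueprint.
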(event `self.ReceiveBeginPlay`
  (`SceneComponent.K2_AddRelativeRotation` (`self.DefaultSceneRoot`) (`KismetMathLibrary.MakeRotator` (`KismetMathLibrary.RandomFloatInRange` -2.0 2.0) (`KismetMathLibrary.RandomFloatInRange` -2.0 2.0) (`KismetMathLibrary.RandomFloatInRange` -2.0 2.0)) false false)
  (`PrimitiveComponent.AddImpulse` (`self.Coll`) (* (`KismetMathLibrary.Conv_RotatorToVector` (`self.K2_GetActorRotation`)) 750.0) "None" false))

(event `self.Coll.OnComponentBeginOverlap`
  (params (OverlappedComponent :type "PrimitiveComponent Object Reference") (OtherActor :type "Actor Object Reference") (OtherComp :type "PrimitiveComponent Object Reference") (OtherBodyIndex :type Integer) (bFromSweep :type Boolean) (SweepResult :type "HitResult Structure (by ref)"))
  (`KismetSystemLibrary.PrintString` "wet" true true (struct :`G` 0.66 :`B` 1.0 :`A` 1.0) 0.1))

(fn `UserConstructionScript`
  (`parent.UserConstructionScript`))