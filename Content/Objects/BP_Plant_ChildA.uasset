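; BP_Plant_ChildA is a BP_Plant variant with plant index 0 that removes itself when spawned too close to certain other plants.
; On BeginPlay it scans plants overlapping its Sphere and flags itself for destruction within a radius-based distance of index 0 or 4 plants.
; Index 4 uses both plants' combined area radii, while index 0 uses half the other's.
; The construction script sets the index and flattens AnchorScaleTemp.
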(event `self.ReceiveBeginPlay`
  (`parent.ReceiveBeginPlay`)
  (for _array_element (`PrimitiveComponent.GetOverlappingActors` (`self.Sphere`) "/Game/Objects/BP_Plant.BP_Plant_C")
    (`/Engine/EditorBlueprintResources/StandardMacros.IsValid` _array_element
      (:`Is Valid`
        (bind _asbp_plant (cast `/Game/Objects/BP_Plant` _array_element))
        (bind _plantindex (`/Game/Objects/BP_Plant.PlantIndex` _asbp_plant))
        (bind _returnvalue (== _plantindex 4))
        (bind _arearadius (`/Game/Objects/BP_Plant.AreaRadius` _asbp_plant))
        (if (and (or (== _plantindex 0) _returnvalue) (< (`KismetMathLibrary.VSize` (- (`self.K2_GetActorLocation` _asbp_plant) (`self.K2_GetActorLocation`))) (* (select `bool` _returnvalue :`false` (/ _arearadius 2.0) :`true` (+ _arearadius (`self.AreaRadius`))) 50.0)))
          (set `self.ToDestroy` true)))))
  (if (`self.ToDestroy`)
    (`self.K2_DestroyActor`)))

(fn `UserConstructionScript`
  (`parent.UserConstructionScript`)
  (set `self.PlantIndex` 0)
  (`SceneComponent.SetRelativeScale3D` (`self.AnchorScaleTemp`) (1.5 1.5 0.3)))