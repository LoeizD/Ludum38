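; BP_SeedVisual is the visual actor for a seed, with a selection circle that can be shown or hidden.
; UpdateLocRot moves and rotates it to a given transform, shifted horizontally by its Offset.
; CircleUpdate turns the AnchorLookAtCamera component toward the BP_HeroN player's camera and sets the circle's visibility.
; It has no active events of its own, so both functions rely on external callers.
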(fn `CircleUpdate`
  (params (bNewVisibility :type Boolean))
  (`SceneComponent.K2_SetWorldRotation` (`self.AnchorLookAtCamera`) (`KismetMathLibrary.FindLookAtRotation` (`SceneComponent.K2_GetComponentLocation` (`self.AnchorLookAtCamera`)) (`SceneComponent.K2_GetComponentLocation` (`/Game/Character/BP_HeroN.Camera` (cast `/Game/Character/BP_HeroN` (`GameplayStatics.GetPlayerPawn` 0) :!pure true)))) false false)
  (`SceneComponent.SetVisibility` (`self.CircleSelection`) bNewVisibility false))

(fn `UpdateLocRot`
  (params (NewLocation :type "Vector Structure") (NewRotation :type "Rotator Structure"))
  (bind (_offset_x _offset_y) (`KismetMathLibrary.BreakVector2D` (`self.Offset`)))
  (`self.K2_SetActorLocationAndRotation` (+ NewLocation (`KismetMathLibrary.MakeVector` _offset_x _offset_y)) NewRotation))

(fn `UserConstructionScript`)