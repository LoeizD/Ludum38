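; BP_Plant_Child2 is a plant variant that inherits its behavior from a parent plant Blueprint.
; Its Construction Script runs the parent's, then sets the plant index, stretches the temporary anchor's scale vertically, and overrides maximum life and the seed spawn time range.
; The event graph holds only disabled placeholder events, so this child differs purely through those construction-time values.
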(fn `UserConstructionScript`
  (`parent.UserConstructionScript`)
  (set `self.PlantIndex` 2)
  (`SceneComponent.SetRelativeScale3D` (`self.AnchorScaleTemp`) (1.0 1.0 1.5))
  (set `self.LifeMax` 10.0)
  (set `self.SeedSpawnTimeMin` 11.0)
  (set `self.SeedSpawnTimeMax` 16.0))